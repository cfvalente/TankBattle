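; Tank projectile actor that physically knocks pawns on impact and then destroys itself.
; When its Sphere component hits a Pawn with a StaticMeshComponent root, it applies an impulse of projectile velocity times Mass to that mesh.
; The impulse is applied at the Sphere's world location rather than at the reported hit point.
; BeginPlay, Tick and the construction script are empty, and the debug prints are unconnected.
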(event `self.Sphere.OnComponentHit`
  (params (HitComponent :type "PrimitiveComponent Object Reference") (OtherActor :type "Actor Object Reference") (OtherComp :type "PrimitiveComponent Object Reference") (NormalImpulse :type "Vector Structure") (Hit :type "HitResult Structure (by ref)"))
  (bind _aspawn (cast `Pawn` OtherActor)
    (:`then`
      (bind _asstatic_mesh_component (cast `StaticMeshComponent` (`self.K2_GetRootComponent` _aspawn))
        (:`then`
          (`PrimitiveComponent.AddImpulseAtLocation` _asstatic_mesh_component (* (`self.GetVelocity`) (`self.Mass`)) (`SceneComponent.K2_GetComponentLocation` HitComponent) "None"))
        (:`CastFailed`
          _)))
    (:`CastFailed`
      _))
  (`self.K2_DestroyActor` self))

(fn `UserConstructionScript`)