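; Projectile Blueprint that switches itself off when its collision mesh hits something.
; On hit, it hides the mesh and disables its collision, except when the hit Pawn is already being destroyed.
; The Pawn root's static mesh and physics checks have no effect, as the velocity-times-mass impulse and debug prints are disconnected.
; The actor itself is never destroyed here, and LaunchBlast is unused.
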(event `self.CollisionMesh.OnComponentHit`
  (params (HitComponent :type "PrimitiveComponent Object Reference") (OtherActor :type "Actor Object Reference") (OtherComp :type "PrimitiveComponent Object Reference") (NormalImpulse :type "Vector Structure") (Hit :type "HitResult Structure (by ref)"))
  (bind _aspawn (cast `Pawn` OtherActor)
    (:`then`
      (if (not (`self.IsActorBeingDestroyed` _aspawn))
        (bind _asstatic_mesh_component (cast `StaticMeshComponent` (`self.K2_GetRootComponent` _aspawn))
          (:`then`
            (if (`SceneComponent.IsSimulatingPhysics` _asstatic_mesh_component "None")
              _
              (else
                _)))
          (:`CastFailed`
            _))
        (`SceneComponent.SetVisibility` (`self.CollisionMesh`) false false :!label _label)
        (`PrimitiveComponent.SetCollisionResponseToAllChannels` (`self.CollisionMesh`) "ECR_Ignore")
        (`PrimitiveComponent.SetCollisionEnabled` (`self.CollisionMesh`) "NoCollision")))
    (:`CastFailed`
      (goto _label))))

(fn `UserConstructionScript`)